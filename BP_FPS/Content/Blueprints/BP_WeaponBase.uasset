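; Base weapon for a first-person shooting range: interacting picks it up if the player has none, attaching it to the arms and enabling weapon input.
; Firing line-traces from the camera, notifying hit targets or, otherwise, the game state.
; Each shot briefly spawns a field-system actor at the impact point and plays sound and montage.
; Reloading draws from the player's typed spare ammo, refilling after a delay and updating the UI.
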(event `/Game/Blueprints/BPI_Interactable.Interact`
  (params (`Player Ref` :type "/Game/FirstPerson/Blueprints/BP_FirstPersonCharacter Object Reference"))
  (bind _firstpersonmesh (`/Game/FirstPerson/Blueprints/BP_FirstPersonCharacter.FirstPersonMesh` (`self.Player Ref`)))
  ;[1 1 1] Interact
  (bind (_owning_player _weapon_picked) (`self.Get Player Info` `Player Ref`))
  (if _weapon_picked
    (`self.Initialize UI` _owning_player)
    (`SceneComponent.K2_AttachToComponent` (`self.SM_Rifle_01`) _firstpersonmesh "GripPoint" "SnapToTarget" "SnapToTarget" "SnapToTarget" true)
    (bind _asfirst_person_anim_bp (cast `/Game/FirstPersonArms/Animations/FirstPerson_AnimBP` (`SkeletalMeshComponent.GetAnimInstance` _firstpersonmesh)))
    (set `/Game/FirstPersonArms/Animations/FirstPerson_AnimBP.HasRifle` true _asfirst_person_anim_bp)
    (`self.Apply Position Offset`)
    (bind _asbp_first_person_player_controller (cast `/Game/FirstPerson/Blueprints/BP_FirstPersonPlayerController` (`Pawn.GetController` (`self.Player Ref`))))
    (bind _returnvalue (pcsubsystem `EnhancedInputLocalPlayerSubsystem` _asbp_first_person_player_controller))
    (`/Engine/EditorBlueprintResources/StandardMacros.IsValid` _returnvalue
      (:`Is Valid`
        (`EnhancedInputSubsystemInterface.AddMappingContext` _returnvalue "/Game/FirstPerson/Input/IMC_Weapons.IMC_Weapons" 0 (struct))
        (`self.EnableInput` (`GameplayStatics.GetPlayerController` 0))))))

(event `EnhancedInput|/Game/FirstPerson/Input/Actions/IA_Shoot`
  (params (ActionValue :type Boolean) (ElapsedSeconds :type "Float (double-precision)") (TriggeredSeconds :type "Float (double-precision)") (InputAction :type "InputAction Object Reference" :default "/Game/FirstPerson/Input/Actions/IA_Shoot.IA_Shoot"))
  (bind (_start_pos _end_pos) (`self.Calculate Bullet Path` 10000.0))
  (bind _player_ref (`self.Player Ref`))
  ;[1 1 1] Fire
  (:`Triggered`
    (if (`self.Can Fire?`)
      (bind _outhit (`KismetSystemLibrary.LineTraceSingleForObjects` _start_pos _end_pos (`|MakeArray` "ObjectTypeQuery1" "ObjectTypeQuery2" "ObjectTypeQuery6" :!type "EObjectTypeQuery Enum")))
      (bind (_bblockinghit _binitialoverlap _time _distance _location _impactpoint _normal _impactnormal _physmat _hitactor) (`GameplayStatics.BreakHitResult` _outhit))
      (bind _asbp_target_base (cast `/Game/Blueprints/BP_TargetBase` _hitactor)
        (:`then`
          (`/Game/Blueprints/BP_TargetBase.Target Hit` _asbp_target_base)
          (`/Game/Blueprints/BP_TargetBase.Enable Physics` _asbp_target_base))
        (:`CastFailed`
          (bind _asbp_shooting_range_gamestate (cast `/Game/Blueprints/BP_ShootingRangeGamestate` (`GameplayStatics.GetGameState`)))
          (`/Game/Blueprints/BP_ShootingRangeGamestate.Round Fired` _asbp_shooting_range_gamestate)))
      (`/Engine/EditorBlueprintResources/StandardMacros.DecrementInt` (`self.Rounds in Mag`)
        (:`  `
          (bind _returnvalue (`|SpawnActorFromClass` "/Engine/EditorResources/FieldNodes/FS_MasterField.FS_MasterField_C" (`KismetMathLibrary.Conv_VectorToTransform` _impactpoint) "Undefined" "MultiplyWithRoot" null null))
          (`/Engine/EditorResources/FieldNodes/FS_MasterField.CE_Trigger` _returnvalue)
          (`self.K2_DestroyActor` _returnvalue)
          (`GameplayStatics.PlaySoundAtLocation` (`self.Fire Sound`) (`self.K2_GetActorLocation` _player_ref) (struct) 1.0 1.0 0.0 null null null null)
          (`AnimInstance.Montage_Play` (`SkeletalMeshComponent.GetAnimInstance` (`/Game/FirstPerson/Blueprints/BP_FirstPersonCharacter.FirstPersonMesh` _player_ref)) "/Game/FirstPersonArms/Animations/FP_Rifle_Shoot_Montage.FP_Rifle_Shoot_Montage" 1.0 "MontageLength" 0.0 true)
          (`/Game/Blueprints/WBP_MainUI.Update Current Weapon Ammo Text` (`/Game/FirstPerson/Blueprints/BP_FirstPersonCharacter.My UI Ref` (`self.Player Ref`)) (`self.Rounds in Mag`)))))))

(event `Attempt Reload`
  (bind (_ammo_amount _has_ammo_already_) (`/Game/FirstPerson/Blueprints/BP_FirstPersonCharacter.Get Spare Ammo Count` (`self.Player Ref`) (`self.Ammo Type`)))
  ;[1 1 1] Reload
  (if (not (`self.Is Reloading?`))
    (if _has_ammo_already_
      (if (`self.Can Reload?` _ammo_amount)
        (bind _rounds_removed (`/Game/FirstPerson/Blueprints/BP_FirstPersonCharacter.Subtract Ammo` (`self.Player Ref`) (`self.Ammo Type`) (`self.Get Rounds Needed Reload`)))
        (`self.Reload` _rounds_removed)))))

(event `EnhancedInput|/Game/Blueprints/IA_Reload`
  (params (ActionValue :type Boolean) (ElapsedSeconds :type "Float (double-precision)") (TriggeredSeconds :type "Float (double-precision)") (InputAction :type "InputAction Object Reference" :default "/Game/Blueprints/IA_Reload.IA_Reload"))
  ;[1 1 1] Reload
  (:`Triggered`
    (`self.Attempt Reload`)))

(fn `Apply Position Offset`
  (`self.K2_SetActorRelativeTransform` (`KismetMathLibrary.MakeTransform` (`self.Location Offset`) (`self.Rotation Offset`))))

(fn `Calculate Bullet Path`
  (params (`Max Bullet Range` :type "Float (double-precision)"))
  (returns (`Start Pos` :type "Vector Structure") (`End Pos` :type "Vector Structure"))
  (bind _firstpersoncamera (`/Game/FirstPerson/Blueprints/BP_FirstPersonCharacter.FirstPersonCamera` (`self.Player Ref`)))
  (bind _returnvalue (`SceneComponent.K2_GetComponentLocation` _firstpersoncamera))
  (return _returnvalue (+ _returnvalue (* (`SceneComponent.GetForwardVector` _firstpersoncamera) `Max Bullet Range`))))

(fn `Can Fire?`
  (returns (Result :type Boolean))
  (return (and (not (`self.Is Reloading?`)) (>= (`self.Rounds in Mag`) 1))))

(fn `Can Reload?`
  (params (`Player Ammo Count` :type Integer))
  (returns (Result :type Boolean))
  (return (and (>= `Player Ammo Count` 1) (< (`self.Rounds in Mag`) (`self.Mag Capacity`)))))

(fn `Get Player Info`
  (params (Player :type "/Game/FirstPerson/Blueprints/BP_FirstPersonCharacter Object Reference"))
  (returns (`Owning Player` :type "/Game/FirstPerson/Blueprints/BP_FirstPersonCharacter Object Reference") (`Weapon Picked` :type Boolean))
  (locals (`Has Weapon Local` :type Boolean :default false))
  (bind _output_get (set `local.Has Weapon Local` (`/Game/FirstPerson/Blueprints/BP_FirstPersonCharacter.Has Weapon?` Player)))
  (if _output_get
    (set `local.Has Weapon Local` false)
    (else
      (bind _output_get_2 (set `/Game/FirstPerson/Blueprints/BP_FirstPersonCharacter.Has Weapon?` true Player))
      (set `local.Has Weapon Local` _output_get_2)
      (set `/Game/FirstPerson/Blueprints/BP_FirstPersonCharacter.Weapon Ref` self Player)
      (`/Engine/EditorBlueprintResources/StandardMacros.DoOnce` false
        (:`Completed`
          _))))
  (return Player (`local.Has Weapon Local`)))

(fn `Get Rounds Needed Reload`
  (returns (`Rounds Needed` :type Integer))
  (return (- (`self.Mag Capacity`) (`self.Rounds in Mag`))))

(fn `Initialize UI`
  (params (Player :type "/Game/FirstPerson/Blueprints/BP_FirstPersonCharacter Object Reference"))
  (bind _output_get (set `self.Player Ref` Player))
  (bind _my_ui_ref (`/Game/FirstPerson/Blueprints/BP_FirstPersonCharacter.My UI Ref` _output_get))
  (`/Game/Blueprints/WBP_MainUI.Update Current Weapon Ammo Text` _my_ui_ref (`self.Rounds in Mag`))
  (`/Game/Blueprints/WBP_MainUI.Update Spare Ammo Text` _my_ui_ref (`self.Ammo Type`)))

(fn `UserConstructionScript`)