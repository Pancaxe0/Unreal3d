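; Shooting range game state that tracks a timed course: elapsed time, shots fired, targets hit and accuracy.
; BeginPlay counts BP_TargetBase actors and sets game-only input; StartCourse starts the Tick-driven timer once.
; While timing, TargetHit also logs a round, updating the accuracy string, and decrements remaining targets.
; At zero targets, FinishCourse stops the timer, then after a delay pauses and switches to cursor-driven UI input.
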(event `Start Course`
  (`/Engine/EditorBlueprintResources/StandardMacros.DoOnce` false
    (:`Completed`
      (set `self.TimerStarted?` true))))

(event `Finish Course`
  (bind _returnvalue (`GameplayStatics.GetPlayerController` 0))
  (set `self.TimerStarted?` false)
  (`KismetSystemLibrary.Delay` 1.0)
  (`GameplayStatics.SetGamePaused` true)
  (set `PlayerController.bShowMouseCursor` true _returnvalue)
  (`WidgetBlueprintLibrary.SetInputMode_UIOnlyEx` _returnvalue null))

(event `Count Targets on Course`
  (bind _outactors (`GameplayStatics.GetAllActorsOfClass` "/Game/Blueprints/BP_TargetBase.BP_TargetBase_C"))
  (set `self.TargetsRemaining` (`KismetArrayLibrary.Array_Length` _outactors)))

(event `Check If Course Complete`
  (if (== (`self.TargetsRemaining`) 0)
    (`self.Finish Course`)))

(event `Calculate Accuracy`
  (if (`self.TimerStarted?`)
    (set `self.CurrentAccuracy` (`KismetStringLibrary.Concat_StrStr` (`KismetStringLibrary.Conv_DoubleToString` (* (/ (`KismetMathLibrary.Conv_IntToDouble` (`self.TotalTargetsHit`)) (`KismetMathLibrary.Conv_IntToDouble` (`self.TotalRoundsFired`))) 100.0)) "%"))))

(event `Round Fired`
  (if (`self.TimerStarted?`)
    (`/Engine/EditorBlueprintResources/StandardMacros.IncrementInt` (`self.TotalRoundsFired`)
      (:`  `
        (`self.Calculate Accuracy`)))))

(event `Target Hit`
  (if (`self.TimerStarted?`)
    (`/Engine/EditorBlueprintResources/StandardMacros.IncrementInt` (`self.TotalTargetsHit`)
      (:`  `
        (`/Engine/EditorBlueprintResources/StandardMacros.DecrementInt` (`self.TargetsRemaining`)
          (:`  `
            (`self.Round Fired`)
            (`self.Check If Course Complete`)))))))

(event `Increase Timer`
  (params (`Time to Add` :type "Float (double-precision)"))
  (bind _output_get (set `self.TotalTimePassed` (+ `Time to Add` (`self.TotalTimePassed`))))
  (set `self.RoundedTime` (`KismetStringLibrary.Conv_IntToString` (`KismetMathLibrary.Round` _output_get))))

(event `self.ReceiveTick`
  (params (DeltaSeconds :type "Float (single-precision)"))
  (if (`self.TimerStarted?`)
    (`self.Increase Timer` DeltaSeconds)))

(event `self.ReceiveBeginPlay`
  (`self.Count Targets on Course`)
  (`GameplayStatics.SetGamePaused` false)
  (`WidgetBlueprintLibrary.SetInputMode_GameOnly` (`GameplayStatics.GetPlayerController` 0)))

(fn `UserConstructionScript`)